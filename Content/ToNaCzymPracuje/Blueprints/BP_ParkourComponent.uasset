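; Parkour component for a Character owner that adds vault, mantle and slide moves.
; TryParkour traces forward and down, then picks by ledge height a launched vault or a Tick-lerped mantle with movement disabled.
; Slides crouch, launch, swap friction and braking, and switch BP_PlayerCharacter's camera target until a timer restores them.
; TrySlide only flags IsSliding when fast and grounded, calling StartSlide only if already flagged.
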(event Custom|StartMantle
  (params (TargetLocation :type Vector))
  (Variables|Default|SetbIsParkouring true)
  (Pawn|Components|CharacterMovement|DisableMovement (Variables|/Script/Engine.Character|GetCharacterMovement (CallFunction|GetOwnerCharacter)))
  (Variables|Default|SetMantleElapsed 0.0)
  (bind _output_get (Variables|Default|SetMantleStart (Transformation|GetActorLocation (CallFunction|GetOwnerCharacter))))
  (bind _output_get_2 (Variables|Default|SetMantleTarget TargetLocation)))

(event Custom|FinishMantle
  (bind _ownercharacter (CallFunction|GetOwnerCharacter))
  (Transformation|SetActorLocation _ownercharacter (Variables|Default|GetMantleTarget) false true)
  (Pawn|Components|CharacterMovement|SetMovementMode (Variables|/Script/Engine.Character|GetCharacterMovement _ownercharacter) "MOVE_Walking" 0)
  (Variables|Default|SetbIsParkouring false))

(event Custom|StartSlide
  (bind _ownercharacter (CallFunction|GetOwnerCharacter))
  (bind _charactermovement (Variables|/Script/Engine.Character|GetCharacterMovement _ownercharacter))
  (Variables|Default|SetSlideElapsed 0.0)
  (Variables|Default|SetIsSliding true)
  (bind _asbp_player_character (Utilities|Casting|CastToBP_PlayerCharacter (CallFunction|GetOwnerCharacter)))
  (Default|SetSlideCameraTarget _asbp_player_character true)
  (Variables|Default|SetSavedMaxWalkSpeed (Variables|/Script/Engine.CharacterMovementComponent|GetMaxWalkSpeed _charactermovement))
  (Variables|Default|SetSavedGroundFriction (Variables|/Script/Engine.CharacterMovementComponent|GetGroundFriction _charactermovement))
  (Variables|Default|SetSavedBrakingDecel (Variables|/Script/Engine.CharacterMovementComponent|GetBrakingDecelerationWalking _charactermovement))
  (Variables|/Script/Engine.CharacterMovementComponent|SetGroundFriction _charactermovement (Variables|Default|GetSlideGroundFriction))
  (Variables|/Script/Engine.CharacterMovementComponent|SetBrakingDecelerationWalking _charactermovement (Variables|Default|GetSlideBrakingDecel))
  (Character|Crouch _ownercharacter)
  (Character|LaunchCharacter _ownercharacter (* (Transformation|GetActorForwardVector _ownercharacter) (Variables|Default|GetSlideLaunchStrength)) true false))

(event Custom|FinishSlide
  (bind _ownercharacter (CallFunction|GetOwnerCharacter))
  (bind _charactermovement (Variables|/Script/Engine.Character|GetCharacterMovement _ownercharacter))
  (Variables|Default|SetSlideElapsed 0.0)
  (Variables|Default|SetIsSliding false)
  (bind _asbp_player_character (Utilities|Casting|CastToBP_PlayerCharacter (CallFunction|GetOwnerCharacter)))
  (Default|SetSlideCameraTarget _asbp_player_character false)
  (Character|UnCrouch _ownercharacter)
  (Variables|/Script/Engine.CharacterMovementComponent|SetMaxWalkSpeed _charactermovement (Variables|Default|GetSavedMaxWalkSpeed))
  (Variables|/Script/Engine.CharacterMovementComponent|SetGroundFriction _charactermovement (Variables|Default|GetSavedGroundFriction))
  (Variables|/Script/Engine.CharacterMovementComponent|SetBrakingDecelerationWalking _charactermovement (Variables|Default|GetSavedBrakingDecel))
  (Variables|Default|SetIsSliding false)
  (Variables|Default|SetSlideElapsed 0.0))

(event EventTick
  (params (DeltaSeconds :type Float%20%28single-precision%29))
  (Utilities|FlowControl|Sequence
    (:then_0
      (if (Variables|Default|GetbIsParkouring)
        (Variables|Default|SetMantleElapsed (+ (Variables|Default|GetMantleElapsed) DeltaSeconds))
        (Transformation|SetActorLocation (CallFunction|GetOwnerCharacter) (Math|Vector|Lerp(Vector) (stale Custom|StartMantle _output_get) (stale Custom|StartMantle _output_get_2) (Math|Float|Clamp(Float) (/ (+ (Variables|Default|GetMantleElapsed) DeltaSeconds) (Variables|Default|GetMantleDuration)))) false false)
        (if (>= (Variables|Default|GetMantleElapsed) (Variables|Default|GetMantleDuration))
          (CallFunction|FinishMantle))))
    (:then_1
      (if (Variables|Default|GetIsSliding)
        (Variables|Default|SetSlideElapsed (+ (Variables|Default|GetSlideElapsed) DeltaSeconds))
        (if (>= (Variables|Default|GetSlideElapsed) (Variables|Default|GetSlideDuration))
          (CallFunction|FinishSlide))))))

(fn TryParkour
  (bind _ownercharacter (CallFunction|GetOwnerCharacter))
  (bind _ownercharacter_2 (CallFunction|GetOwnerCharacter))
  (bind _ownercharacter_3 (CallFunction|GetOwnerCharacter))
  (bind _returnvalue (Transformation|GetActorLocation _ownercharacter_3))
  (bind _returnvalue_2 (+ _returnvalue "0.000000,0.000000,5.000000" ""))
  (if (Variables|Default|GetbIsParkouring)
    (return)
    (else
      (bind (_outhit _returnvalue_3) (Collision|LineTraceByChannel _returnvalue_2 (+ _returnvalue_2 (* (Transformation|GetActorForwardVector _ownercharacter_3) (Variables|Default|GetTraceDistance)) "") "TraceTypeQuery1" false 0 "ForDuration"))
      (if _returnvalue_3
        (bind (_outhit_2 _returnvalue_4) (Collision|LineTraceByChannel (+ (.ImpactPoint (Collision|BreakHitResult _outhit)) "0.000000,0.000000,250.000000") (+ (+ (.ImpactPoint (Collision|BreakHitResult _outhit)) "0.000000,0.000000,250.000000") "0.000000,0.000000,-350.000000") "TraceTypeQuery1" false 0 "ForDuration"))
        (if _returnvalue_4
          (Variables|Default|SetMantleTopZ (.Z (Math|Vector|BreakVector (.Location (Collision|BreakHitResult _outhit_2)))))
          (if (Math|Float|InRange(Float) (- (.Z (Math|Vector|BreakVector (.Location (Collision|BreakHitResult _outhit_2)))) (- (.Z (Math|Vector|BreakVector (Transformation|GetActorLocation _ownercharacter_2))) (Components|Capsule|GetScaledCapsuleHalfHeight (Variables|/Script/Engine.Character|GetCapsuleComponent _ownercharacter_2)))) (Variables|Default|GetMinVaultHeight) (Variables|Default|GetMaxVaultHeight)) ; true = vault
            (Development|PrintString "vault")
            (if (AI|Components|NavMovement|IsFalling (Variables|/Script/Engine.Character|GetCharacterMovement (CallFunction|GetOwnerCharacter)))
              (return)
              (else
                (Character|LaunchCharacter _ownercharacter (+ (* (Math|Vector|GetForwardVector (Math|Rotator|MakeRotator 0.0 0.0 (.Yaw (Math|Rotator|BreakRotator (Pawn|GetControlRotation (Pawn|GetController _ownercharacter) :!class /Script/Engine.Controller))))) (Variables|Default|GetVaultForwardStrength)) (Math|Vector|MakeVector 0.0 0.0 (Variables|Default|GetVaultUpStrength))) true true)))
            (elif (Math|Float|InRange(Float) (- (.Z (Math|Vector|BreakVector (.Location (Collision|BreakHitResult _outhit_2)))) (- (.Z (Math|Vector|BreakVector (Transformation|GetActorLocation _ownercharacter_2))) (Components|Capsule|GetScaledCapsuleHalfHeight (Variables|/Script/Engine.Character|GetCapsuleComponent _ownercharacter_2)))) (Variables|Default|GetMinMantleHeight) (Variables|Default|GetMaxMantleHeight)) ; true = mantle
              (Development|PrintString "Mantle")
              (Variables|Default|SetbIsParkouring true)
              (Variables|Default|SetMantleStart (Transformation|GetActorLocation (CallFunction|GetOwnerCharacter)))
              (Variables|Default|SetMantleTarget (Math|Vector|MakeVector (.X (Math|Vector|BreakVector (+ (Variables|Default|GetMantleStart) (* (Transformation|GetActorForwardVector (CallFunction|GetOwnerCharacter)) (Variables|Default|GetMantleForwardOffset))))) (.Y (Math|Vector|BreakVector (+ (Variables|Default|GetMantleStart) (* (Transformation|GetActorForwardVector (CallFunction|GetOwnerCharacter)) (Variables|Default|GetMantleForwardOffset))))) (+ (+ (Variables|Default|GetMantleTopZ) (Components|Capsule|GetScaledCapsuleHalfHeight (Variables|/Script/Engine.Character|GetCapsuleComponent (CallFunction|GetOwnerCharacter)))) (Variables|Default|GetMantleUpOffset))))
              (CallFunction|StartMantle (Variables|Default|GetMantleTarget))
              (else
                (Development|PrintString "None"))))
          (else
            (return)))
        (else
          (Development|PrintString "No front hit")
          (return))))))

(fn TrySlide
  (bind _ownercharacter (CallFunction|GetOwnerCharacter))
  (if (Variables|Default|GetbIsParkouring)
    (return)
    (elif (Variables|Default|GetIsSliding)
      (CallFunction|StartSlide)
      (return)
      (elif (AI|Components|NavMovement|IsFalling (Variables|/Script/Engine.Character|GetCharacterMovement _ownercharacter))
        (return)
        (elif (>= (Math|Vector|VectorLengthXY (Transformation|GetVelocity _ownercharacter)) (Variables|Default|GetSlideMinSpeed))
          (Variables|Default|SetIsSliding true)
          (return)
          (else
            (return)))))))

(fn GetOwnerCharacter
  (bind _ascharacter (Utilities|Casting|CastToCharacter (Components|GetOwner)))
  (return _ascharacter))

(fn CustomEvent)